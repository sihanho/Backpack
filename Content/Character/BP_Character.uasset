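; BP_Character is a character Blueprint that gives the player a backpack screen toggled with the B key.
; The first press creates the BP_Backpack widget, caches it and adds it to the viewport; later presses remove or re-add that same instance.
; GetBackpackItems exposes the item list held by the ACBackpack component.
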(event `Key|B`
  (params (Key :type "Key Structure"))
  (:`Pressed`
    (`/Engine/EditorBlueprintResources/StandardMacros.IsValid` (`self.BP_BackPack`)
      (:`Is Valid`
        (if (`Widget.IsInViewport` (`self.BP_BackPack`))
          (`Widget.RemoveFromParent` (`self.BP_BackPack`))
          (else
            (`UserWidget.AddToViewport` (`self.BP_BackPack`) 0 :!label _label))))
      (:`Is Not Valid`
        (bind _returnvalue (`|CreateWidget` "/Game/Widgets/BP_Backpack.BP_Backpack_C"))
        (set `self.BP_BackPack` _returnvalue)
        (goto _label)))))

(fn `GetBackpackItems`
  (returns (Items :type "Array of /Game/Struct_BackpackItems Structure"))
  (return (`/Game/AC_Backpack.GetItems` (`self.AC_Backpack`))))

(fn `UserConstructionScript`)